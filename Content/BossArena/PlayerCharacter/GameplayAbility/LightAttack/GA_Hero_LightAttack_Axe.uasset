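; GA_Hero_LightAttack_Axe is the hero's axe light attack ability, adding a slash projectile while Rage is active.
; Activation defers to the parent ability, while WhileRageActive waits for the SpawnProjectile gameplay event.
; On that event it spawns BP_Projectile_HeroSlash at the weapon's RageSlashSocket, taking roll from the socket and yaw from hero facing.
; The projectile carries a light-attack damage spec built from level-scaled weapon damage and a fixed combo count.
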(event `self.K2_ActivateAbility`
  (`parent.K2_ActivateAbility`))

(event `self.WhileRageActive`
  (bind _returnvalue (`self.GetHeroCharacterFromActorInfo`))
  (bind (_returnvalue_roll _returnvalue_pitch _returnvalue_yaw) (`KismetMathLibrary.BreakRotator` (`KismetMathLibrary.MakeRotFromX` (`Actor.GetActorForwardVector` (`self.GetHeroCharacterFromActorInfo`)))))
  (bind _returnvalue_2 (`SceneComponent.GetSocketTransform` (`BAWeaponBase.WeaponMesh` (`HeroCombatComponent.GetHeroCurrentEquippedWeapon` (`self.GetHeroCombatComponentFromActorInfo`))) "RageSlashSocket" "RTS_World"))
  (`AbilityTask_WaitGameplayEvent.WaitGameplayEvent` (struct :`TagName` "Shared.Event.SpawnProjectile") null
    (:`EventReceived`
      (`|SpawnActorFromClass` "/Game/BossArena/PlayerCharacter/BP_Projectile_HeroSlash.BP_Projectile_HeroSlash_C" (`KismetMathLibrary.MakeTransform` (.location _returnvalue_2) (`KismetMathLibrary.MakeRotator` (.roll (.rotation _returnvalue_2)) 0.0 _returnvalue_yaw)) "Undefined" "MultiplyWithRoot" _returnvalue (`self.MakeHeroDamageEffectSpecHandle` "/Game/BossArena/Shared/GameplayEffect/GE_Shared_DealDamage.GE_Shared_DealDamage_C" (`HeroCombatComponent.GetHeroCurrentEquippedWeaponDamageAtLevel` (`self.GetHeroCombatComponentFromActorInfo`) (`KismetMathLibrary.Conv_IntToDouble` (`self.GetAbilityLevel`))) (struct :`TagName` "Player.SetByCaller.AttackType.Light") 3) _returnvalue))))