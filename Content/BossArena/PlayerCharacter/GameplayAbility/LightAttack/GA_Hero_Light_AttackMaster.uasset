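; Master hero light-attack gameplay ability that plays a combo montage chain, with an empty rage hook.
; Each activation advances the combo counter; a JumpToFinisher tag, added on the penultimate step, selects the final montage.
; Melee-hit events apply weapon- and combo-based damage, a sound cue, hit react and rage gain.
; A continue event stops the montage early, and a short timer after ability end resets the combo.
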(event `self.K2_ActivateAbility`
  (`KismetSystemLibrary.K2_ClearAndInvalidateTimerHandle` (`self.ComboCountResetTimerHandle`))
  (`BAFunctionLibrary.BP_DoesActorHaveTag` (`self.GetHeroCharacterFromActorInfo`) (struct :`TagName` "Player.Status.JumpToFinisher")
    (:`Yes`
      (set `self.CurrentLightAttackCombatCount` (`BlueprintMapLibrary.Map_Length` (`self.AttackMontagesMap`))))
    (:`No`
      (set `self.Used Combo Count` (`self.CurrentLightAttackCombatCount`))))
  (`AbilityTask_PlayMontageAndWait.CreatePlayMontageAndWaitProxy` "None" (`BlueprintMapLibrary.Map_Find` (`self.AttackMontagesMap`) (`self.CurrentLightAttackCombatCount`))
    (:`then`
      (`|ExecutionSequence`
        (:`then_0`
          (bind (_asynctaskproxy _payload) (`AbilityTask_WaitGameplayEvent.WaitGameplayEvent` (struct :`TagName` "Shared.Event.MeleeHit") null)
            (:`EventReceived`
              (`self.HandleApplyDamage` _payload))))
        (:`then_1`
          (`AbilityTask_WaitGameplayEvent.WaitGameplayEvent` (struct :`TagName` "Player.Event.Continue.Attack") null
            (:`EventReceived`
              (`self.MontageStop` -1.0))))
        (:`then_2`
          (if (== (`self.CurrentLightAttackCombatCount`) (`BlueprintMapLibrary.Map_Length` (`self.AttackMontagesMap`)))
            (`self.ResetAttackComboCount`)
            (else
              (if (== (`self.CurrentLightAttackCombatCount`) (- (`BlueprintMapLibrary.Map_Length` (`self.AttackMontagesMap`)) 1))
                (`BAFunctionLibrary.AddGameplayTagToActorIfNone` (`self.GetHeroCharacterFromActorInfo`) (struct :`TagName` "Player.Status.JumpToFinisher")))
              (`/Engine/EditorBlueprintResources/StandardMacros.IncrementInt` (`self.CurrentLightAttackCombatCount`)))))
        (:`then_3`
          (`BAFunctionLibrary.BP_DoesActorHaveTag` (`self.GetHeroCharacterFromActorInfo`) (struct :`TagName` "Player.Status.Rage.Active")
            (:`Yes`
              (`self.WhileRageActive`))))))
    (:`OnCompleted`
      (`self.K2_EndAbility` :!label _label)
      (bind _returnvalue (`KismetSystemLibrary.K2_SetTimerDelegate` (delegate `ResetAttackComboCount`) 0.3))
      (set `self.ComboCountResetTimerHandle` _returnvalue))
    (:`OnBlendOut`
      (goto _label))
    (:`OnInterrupted`
      (goto _label))
    (:`OnCancelled`
      (goto _label))))

(event `WhileRageActive`)

(event `ResetAttackComboCount`
  (set `self.CurrentLightAttackCombatCount` 1)
  (`BAFunctionLibrary.RemoveGameplayTagFromActorIfFound` (`self.GetHeroCharacterFromActorInfo`) (struct :`TagName` "Player.Status.JumpToFinisher")))

(fn `HandleApplyDamage`
  (params (GameplayEventData :type "GameplayEventData Structure (by ref)"))
  (locals (LocalTargetActor :type "Actor Object Reference"))
  (bind (_eventtag _instigator _target) (break `GameplayEventData` GameplayEventData))
  (set `local.LocalTargetActor` _target)
  (`self.K2_ExecuteGameplayCue` (`self.WeaponHitSoundGameplayCueTag`))
  (`self.BP_ApplyEffectSpecHandleToTarget` _target (`self.MakeHeroDamageEffectSpecHandle` "/Game/BossArena/Shared/GameplayEffect/GE_Shared_DealDamage.GE_Shared_DealDamage_C" (`HeroCombatComponent.GetHeroCurrentEquippedWeaponDamageAtLevel` (`self.GetHeroCombatComponentFromActorInfo`) (`KismetMathLibrary.Conv_IntToDouble` (`self.GetAbilityLevel`))) (struct :`TagName` "Player.SetByCaller.AttackType.Light") (`self.Used Combo Count`))
    (:`Successful`
      (`AbilitySystemBlueprintLibrary.SendGameplayEventToActor` (`local.LocalTargetActor`) (struct :`TagName` "Shared.Event.HitReact") (`local.GameplayEventData`))
      (`self.BP_ApplyGameplayEffectToOwner` "/Game/BossArena/PlayerCharacter/GameplayEffect/GE_Hero_GainRage.GE_Hero_GainRage_C" (`self.GetAbilityLevel`)))))