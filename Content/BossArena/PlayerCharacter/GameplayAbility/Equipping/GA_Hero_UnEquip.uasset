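; Hero gameplay ability that unequips the axe, playing the unequip montage and clearing the equipped weapon tag as it starts.
; On the unequip gameplay event, it snaps the axe to the back socket and calls HandleUnEquipWeapon.
; For local controllers only, that function unlinks weapon anim layers, removes the input mapping context and granted abilities, and refreshes weapon and ability-slot UI.
; The ability ends when the montage completes, blends out, or is interrupted or cancelled.
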(event `self.K2_ActivateAbility`
  (`AbilityTask_PlayMontageAndWait.CreatePlayMontageAndWaitProxy` "None" "/Game/BossArena/PlayerCharacter/Montages/Equip/AM_Hero_Axe_Unequip.AM_Hero_Axe_Unequip"
    (:`then`
      (set `PawnCombatComponent.CurrentEquippedWeaponTag` (struct) (`self.GetHeroCombatComponentFromActorInfo`))
      (`AbilityTask_WaitGameplayEvent.WaitGameplayEvent` (struct :`TagName` "Player.Event.UnEquip.Axe") null
        (:`EventReceived`
          (`Actor.K2_AttachToComponent` (`PawnCombatComponent.GetCharacterCarriedWeaponByTag` (`self.GetHeroCombatComponentFromActorInfo`) (struct :`TagName` "Player.Weapon.Axe")) (`self.GetOwningComponentFromActorInfo`) "AxeBackSocket" "SnapToTarget" "KeepRelative" "KeepWorld" true)
          (`self.HandleUnEquipWeapon` (`HeroCombatComponent.GetHeroCarriedWeaponByTag` (`self.GetHeroCombatComponentFromActorInfo`) (struct :`TagName` "Player.Weapon.Axe"))))))
    (:`OnCompleted`
      (`self.K2_EndAbility` :!label _label))
    (:`OnBlendOut`
      (goto _label))
    (:`OnInterrupted`
      (goto _label))
    (:`OnCancelled`
      (goto _label))))

(fn `HandleUnEquipWeapon`
  (params (`In Weapon to Equip` :type "BAHeroWeapon Object Reference"))
  (locals (CachedHeroWeaponData :type "BAHeroWeaponData Structure"))
  (bind _returnvalue (`self.GetHeroControllerFromActorInfo`))
  (bind _herouicomponent (`BAHeroCharacter.HeroUIComponent` (`self.GetHeroCharacterFromActorInfo`)))
  (set `local.CachedHeroWeaponData` (`BAHeroWeapon.HeroWeaponData` `In Weapon to Equip`))
  (if (`Controller.IsLocalController` (`self.GetHeroControllerFromActorInfo`))
    (`|ExecutionSequence`
      (:`then_0`
        (`SkeletalMeshComponent.UnlinkAnimClassLayers` (`self.GetOwningComponentFromActorInfo`) (`.WeaponAnimLayerToLink` (break `BAHeroWeaponData` (`local.CachedHeroWeaponData`)))))
      (:`then_1`
        (if (`Controller.IsLocalController` _returnvalue)
          (`EnhancedInputSubsystemInterface.RemoveMappingContext` (pcsubsystem `EnhancedInputLocalPlayerSubsystem` _returnvalue) (`.WeaponInputMappingContest` (break `BAHeroWeaponData` (`local.CachedHeroWeaponData`))) (struct))))
      (:`then_2`
        (`BAAbilitySystemComponent.RemovedGrantedHeroWeaponAbilities` (`self.GetBAAbilitySystemFromActorInfo`) (`BAHeroWeapon.GetGrantedAbilitySpecHandles` (`local.In Weapon to Equip`))))
      (:`then_3`
        (`HeroUIComponent.OnEquippedWeaponChanged` _herouicomponent null)
        (for _array_element (`.SpecialWeaponAbilities` (break `BAHeroWeaponData` (`local.CachedHeroWeaponData`)))
          (`HeroUIComponent.OnAbilityIconSlotUpdated` _herouicomponent (`.InputTag` (break `BAHeroSpecialAbilitySet` _array_element)) null))))))