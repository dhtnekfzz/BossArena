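; Base hero Gameplay Ability that equips a carried weapon, selected by tag, during an equip montage.
; A gameplay event attaches the weapon to a socket, runs HandleEquipWeapon and records the equipped tag; montage end or interruption ends the ability.
; HandleEquipWeapon uses the weapon's data to multicast anim layers, add local input mapping and grant abilities, storing handles on the weapon.
; It also updates UI icons, restoring running cooldowns.
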(event `self.K2_ActivateAbility`
  (`AbilityTask_PlayMontageAndWait.CreatePlayMontageAndWaitProxy` "None" (`self.Montage to Play`)
    (:`then`
      (`AbilityTask_WaitGameplayEvent.WaitGameplayEvent` (`self.Event Tag`) null
        (:`EventReceived`
          (`Actor.K2_AttachToComponent` (`PawnCombatComponent.GetCharacterCarriedWeaponByTag` (`self.GetHeroCombatComponentFromActorInfo`) (`self.In Weapon Tag to Get`)) (`self.GetOwningComponentFromActorInfo`) (`self.Socket Name`) "SnapToTarget" "KeepRelative" "KeepWorld" true)
          (`self.HandleEquipWeapon` (`HeroCombatComponent.GetHeroCarriedWeaponByTag` (`self.GetHeroCombatComponentFromActorInfo`) (`self.In Weapon Tag to Get`)))
          (set `PawnCombatComponent.CurrentEquippedWeaponTag` (`self.In Weapon Tag to Get`) (`self.GetHeroCombatComponentFromActorInfo`)))))
    (:`OnCompleted`
      (`self.K2_EndAbility` :!label _label))
    (:`OnBlendOut`
      (goto _label))
    (:`OnInterrupted`
      (goto _label))
    (:`OnCancelled`
      (goto _label))))

(fn `HandleEquipWeapon`
  (params (`In Weapon to Equip` :type "BAHeroWeapon Object Reference"))
  (locals (CachedHeroWeaponData :type "BAHeroWeaponData Structure"))
  (bind _returnvalue (`self.GetHeroControllerFromActorInfo`))
  (bind (_weaponanimlayertolink _weaponinputmappingcontest _defaultweaponabilities _specialweaponabilities _weaponbasedamage _softweaponicontexture) (break `BAHeroWeaponData` (`local.CachedHeroWeaponData`)))
  (bind (_weaponanimlayertolink_2 _weaponinputmappingcontest_2 _defaultweaponabilities_2 _specialweaponabilities_2) (break `BAHeroWeaponData` (`local.CachedHeroWeaponData`)))
  (bind _herouicomponent (`BAHeroCharacter.HeroUIComponent` (`self.GetHeroCharacterFromActorInfo`)))
  (set `local.CachedHeroWeaponData` (`BAHeroWeapon.HeroWeaponData` `In Weapon to Equip`))
  (`|ExecutionSequence`
    (:`then_0`
      (`BAHeroCharacter.Multicast_LinkAnimLayers` (`self.GetHeroCharacterFromActorInfo`) (`.WeaponAnimLayerToLink` (break `BAHeroWeaponData` (`local.CachedHeroWeaponData`)))))
    (:`then_1`
      (if (`Controller.IsLocalPlayerController` _returnvalue)
        (`EnhancedInputSubsystemInterface.AddMappingContext` (pcsubsystem `EnhancedInputLocalPlayerSubsystem` _returnvalue) (`.WeaponInputMappingContest` (break `BAHeroWeaponData` (`local.CachedHeroWeaponData`))) 1 (struct))))
    (:`then_2`
      (bind _outgrantedabilityspechandles (`BAAbilitySystemComponent.GrantHeroWeaponAbilities` (`self.GetBAAbilitySystemFromActorInfo`) _defaultweaponabilities_2 _specialweaponabilities_2 (`self.GetAbilityLevel`)))
      (`BAHeroWeapon.AssignGrantedAbilitySpecHandle` (`local.In Weapon to Equip`) _outgrantedabilityspechandles))
    (:`then_3`
      (`HeroUIComponent.OnEquippedWeaponChanged` _herouicomponent _softweaponicontexture)
      (for _array_element _specialweaponabilities
        (bind (_softabilityiconmaterial _abilitycooldowntag _inputtag) (break `BAHeroSpecialAbilitySet` _array_element))
        (`HeroUIComponent.OnAbilityIconSlotUpdated` _herouicomponent _inputtag _softabilityiconmaterial)
        (bind (_totalcooldowntime _remainingcooldowntime _returnvalue_2) (`self.GetAbilityRemainingCooldownByTag` _abilitycooldowntag))
        (if _returnvalue_2
          (`HeroUIComponent.OnAbilityCooldownBegin` (`BAHeroCharacter.HeroUIComponent` (`self.GetHeroCharacterFromActorInfo`)) _inputtag _totalcooldowntime _remainingcooldowntime))))))