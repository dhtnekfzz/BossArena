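; Hero gameplay ability that equips the carried axe weapon.
; It plays the equip montage and, on the equip gameplay event, snaps the axe to the right-hand socket and marks it as the current equipped weapon.
; HandleEquipWeapon then applies the weapon's data: linking its anim layer, adding its input mapping context, and granting its abilities, storing their spec handles on the weapon.
; The ability ends when the montage finishes or is interrupted.
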(event `self.K2_ActivateAbility`
  (`AbilityTask_PlayMontageAndWait.CreatePlayMontageAndWaitProxy` "None" "/Game/BossArena/PlayerCharacter/Montages/AM_Hero_Axe_Equip.AM_Hero_Axe_Equip"
    (:`then`
      (`AbilityTask_WaitGameplayEvent.WaitGameplayEvent` (struct :`TagName` "Player.Event.Equip.Axe") null
        (:`EventReceived`
          (`Actor.K2_AttachToComponent` (`PawnCombatComponent.GetCharacterCarriedWeaponByTag` (`self.GetHeroCombatComponentFromActorInfo`) (struct :`TagName` "Player.Weapon.Axe")) (`self.GetOwningComponentFromActorInfo`) "AxeRightHandSocket" "SnapToTarget" "KeepRelative" "KeepWorld" true)
          (`self.HandleEquipWeapon` (`HeroCombatComponent.GetHeroCarriedWeaponByTag` (`self.GetHeroCombatComponentFromActorInfo`) (struct :`TagName` "Player.Weapon.Axe")))
          (set `PawnCombatComponent.CurrentEquippedWeaponTag` (struct :`TagName` "Player.Weapon.Axe") (`self.GetHeroCombatComponentFromActorInfo`)))))
    (:`OnCompleted`
      (`self.K2_EndAbility` :!label _label))
    (:`OnBlendOut`
      (goto _label))
    (:`OnInterrupted`
      (goto _label))
    (:`OnCancelled`
      (goto _label))))

(fn `HandleEquipWeapon`
  (params (`In Weapon to Equip` :type "BAHeroWeapon Object Reference"))
  (locals (CachedHeroWeaponData :type "BAHeroWeaponData Structure"))
  (set `local.CachedHeroWeaponData` (`BAHeroWeapon.HeroWeaponData` `In Weapon to Equip`))
  (`|ExecutionSequence`
    (:`then_0`
      (`SkeletalMeshComponent.LinkAnimClassLayers` (`self.GetOwningComponentFromActorInfo`) (`.WeaponAnimLayerToLink` (break `BAHeroWeaponData` (`local.CachedHeroWeaponData`)))))
    (:`then_1`
      (`EnhancedInputSubsystemInterface.AddMappingContext` (pcsubsystem `EnhancedInputLocalPlayerSubsystem` (`self.GetHeroControllerFromActorInfo`)) (`.WeaponInputMappingContest` (break `BAHeroWeaponData` (`local.CachedHeroWeaponData`))) 1 (struct)))
    (:`then_2`
      (bind _outgrantedabilityspechandles (`BAAbilitySystemComponent.GrantHeroWeaponAbilities` (`self.GetBAAbilitySystemFromActorInfo`) (`.DefaultWeaponAbilities` (break `BAHeroWeaponData` (`local.CachedHeroWeaponData`))) (`self.GetAbilityLevel`)))
      (`BAHeroWeapon.AssignGrantedAbilitySpecHandle` (`local.In Weapon to Equip`) _outgrantedabilityspechandles))))