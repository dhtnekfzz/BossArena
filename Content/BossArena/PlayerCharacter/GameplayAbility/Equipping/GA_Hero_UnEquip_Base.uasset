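; Base hero gameplay ability that puts away the currently equipped weapon in the BossArena game.
; It caches and clears the equipped weapon tag, plays a montage, and ends when that montage finishes or is interrupted.
; A gameplay event during the montage snaps the weapon to a socket and calls HandleUnEquipWeapon.
; That function unlinks the weapon's anim layer, removes its input mapping context and granted abilities, and notifies the hero UI.
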(event `self.K2_ActivateAbility`
  (set `self.Current Equipped Weapon Tag` (`PawnCombatComponent.CurrentEquippedWeaponTag` (`self.GetHeroCombatComponentFromActorInfo`)))
  (`AbilityTask_PlayMontageAndWait.CreatePlayMontageAndWaitProxy` "None" (`self.Montage to Play`)
    (:`then`
      (set `PawnCombatComponent.CurrentEquippedWeaponTag` (struct) (`self.GetHeroCombatComponentFromActorInfo`))
      (`AbilityTask_WaitGameplayEvent.WaitGameplayEvent` (`self.Event Tag`) null
        (:`EventReceived`
          (`Actor.K2_AttachToComponent` (`PawnCombatComponent.GetCharacterCarriedWeaponByTag` (`self.GetHeroCombatComponentFromActorInfo`) (`self.Current Equipped Weapon Tag`)) (`self.GetOwningComponentFromActorInfo`) (`self.Socket Name`) "SnapToTarget" "KeepRelative" "KeepWorld" true)
          (`self.HandleUnEquipWeapon` (`HeroCombatComponent.GetHeroCarriedWeaponByTag` (`self.GetHeroCombatComponentFromActorInfo`) (`self.Current Equipped Weapon Tag`))))))
    (:`OnCompleted`
      (`self.K2_EndAbility` :!label _label))
    (:`OnBlendOut`
      (goto _label))
    (:`OnInterrupted`
      (goto _label))
    (:`OnCancelled`
      (goto _label))))

(fn `HandleUnEquipWeapon`
  (params (`In Weapon to Equip` :type "BAHeroWeapon Object Reference"))
  (locals (CachedHeroWeaponData :type "BAHeroWeaponData Structure"))
  (bind _herouicomponent (`BAHeroCharacter.HeroUIComponent` (`self.GetHeroCharacterFromActorInfo`)))
  (set `local.CachedHeroWeaponData` (`BAHeroWeapon.HeroWeaponData` `In Weapon to Equip`))
  (`|ExecutionSequence`
    (:`then_0`
      (`SkeletalMeshComponent.UnlinkAnimClassLayers` (`self.GetOwningComponentFromActorInfo`) (`.WeaponAnimLayerToLink` (break `BAHeroWeaponData` (`local.CachedHeroWeaponData`)))))
    (:`then_1`
      (`EnhancedInputSubsystemInterface.RemoveMappingContext` (pcsubsystem `EnhancedInputLocalPlayerSubsystem` (`self.GetHeroControllerFromActorInfo`)) (`.WeaponInputMappingContest` (break `BAHeroWeaponData` (`local.CachedHeroWeaponData`))) (struct)))
    (:`then_2`
      (`BAAbilitySystemComponent.RemovedGrantedHeroWeaponAbilities` (`self.GetBAAbilitySystemFromActorInfo`) (`BAHeroWeapon.GetGrantedAbilitySpecHandles` (`local.In Weapon to Equip`))))
    (:`then_3`
      (`HeroUIComponent.OnEquippedWeaponChanged` _herouicomponent null)
      (for _array_element (`.SpecialWeaponAbilities` (break `BAHeroWeaponData` (`local.CachedHeroWeaponData`)))
        (`HeroUIComponent.OnAbilityIconSlotUpdated` _herouicomponent (`.InputTag` (break `BAHeroSpecialAbilitySet` _array_element)) null)))))