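; Master gameplay ability for the hero's heavy attack combo, playing a montage chosen from a map by the current combo count.
; Each activation clears the reset timer, skips to the last montage if the hero has the JumpToFinisher tag, then advances the count, or resets it after the finisher.
; When the montage ends or is interrupted, the ability ends and starts a short timer that resets the combo and removes that tag.
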(event `self.K2_ActivateAbility`
  (`KismetSystemLibrary.K2_ClearAndInvalidateTimerHandle` (`self.ComboCountResetTimerHandle`))
  (`BAFunctionLibrary.BP_DoesActorHaveTag` (`self.GetHeroCharacterFromActorInfo`) (struct :`TagName` "Player.Status.JumpToFinisher")
    (:`Yes`
      (set `self.CurrentHeavyAttackCombatCount` (`BlueprintMapLibrary.Map_Length` (`self.AttackMontagesMap`))))
    (:`No`
      _))
  (`AbilityTask_PlayMontageAndWait.CreatePlayMontageAndWaitProxy` "None" (`BlueprintMapLibrary.Map_Find` (`self.AttackMontagesMap`) (`self.CurrentHeavyAttackCombatCount`))
    (:`then`
      (`|ExecutionSequence`
        (:`then_0`
          (if (== (`self.CurrentHeavyAttackCombatCount`) (`BlueprintMapLibrary.Map_Length` (`self.AttackMontagesMap`)))
            (`self.ResetHeavyAttackComboCount`)
            (else
              (`/Engine/EditorBlueprintResources/StandardMacros.IncrementInt` (`self.CurrentHeavyAttackCombatCount`)))))))
    (:`OnCompleted`
      (`self.K2_EndAbility` :!label _label)
      (bind _returnvalue (`KismetSystemLibrary.K2_SetTimerDelegate` (delegate `ResetHeavyAttackComboCount`) 0.3))
      (set `self.ComboCountResetTimerHandle` _returnvalue))
    (:`OnBlendOut`
      (goto _label))
    (:`OnInterrupted`
      (goto _label))
    (:`OnCancelled`
      (goto _label))))

(event `ResetHeavyAttackComboCount`
  (set `self.CurrentHeavyAttackCombatCount` 1)
  (`BAFunctionLibrary.RemoveGameplayFromActorIfFound` (`self.GetHeroCharacterFromActorInfo`) (struct :`TagName` "Player.Status.JumpToFinisher")))