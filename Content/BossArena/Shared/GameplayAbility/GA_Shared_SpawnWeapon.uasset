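; Shared gameplay ability that spawns a configurable weapon actor and attaches it to the avatar pawn.
; On activation it spawns the weapon with the pawn as owner and instigator, then attaches it to a socket on the owning component.
; It registers the weapon by tag, optionally as equipped, with the pawn combat component.
; The ability ends only when the spawn succeeds, as an invalid spawn has no handling.
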(event `self.K2_ActivateAbility`
  (bind `_as폰` (cast `Pawn` (`self.GetAvatarActorFromActorInfo`) :!pure true))
  (bind _returnvalue (`|SpawnActorFromClass` (`self.Weapon Class to Spawn`) (`KismetMathLibrary.MakeTransform` (0.0 0.0 0.0)) "Undefined" "MultiplyWithRoot" `_as폰` `_as폰`))
  (`/Engine/EditorBlueprintResources/StandardMacros.IsValid` _returnvalue
    (:`Is Valid`
      (`Actor.K2_AttachToComponent` _returnvalue (`self.GetOwningComponentFromActorInfo`) (`self.Socket Name to Attach To`) "SnapToTarget" "KeepRelative" "KeepWorld" true)
      (`PawnCombatComponent.RegisterSpawnedWeapon` (`self.GetPawnCombatComponentFromActorInfo`) (`self.In Weapon Tag to Register`) _returnvalue (`self.Register as Equipped Weapon`))
      (`self.K2_EndAbility`))))