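; Survival game mode Blueprint for the boss arena, intended to present wave and match state changes, though its event handlers are currently empty.
; Disconnected logic switches on state to show wave text, or fade the camera and async-load win and lose screens.
; Other unwired fragments show a boss countdown and fire a new-wave GameplayCue.
; Two helper functions create wave text widgets and start their timers, called only from that dead logic.
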(event `self.ReceiveBeginPlay`)

(event `OnSurvivalGameModeStateChanged_이벤트`
  (params (CurrentState :type "EBASurvivalGameModeState Enum" :default "WaitSpawnNewWave")))

(fn `CreateWaveWidgetWithCountDown`
  (params (`Text Content to Display` :type Text) (InTotalCountDownTime :type "Float (single-precision)"))
  (bind _returnvalue (`|CreateWidget` "/Game/BossArena/Widgets/GameModeWidgets/WBP_WaveTextWithCountDown.WBP_WaveTextWithCountDown_C"))
  (`UserWidget.AddToViewport` _returnvalue 0)
  (`TextBlock.SetText` (`/Game/BossArena/Widgets/GameModeWidgets/WBP_WaveTextWithCountDown.TextBlock_WaveText` _returnvalue) (`local.Text Content to Display`))
  (`/Game/BossArena/Widgets/GameModeWidgets/WBP_WaveTextWithCountDown.StartCountDown` _returnvalue (`local.InTotalCountDownTime`)))

(fn `CreateWaveWidgetWithNoCountDown`
  (params (`Text Content to Display` :type Text) (InTotalCountDownTime :type "Float (single-precision)"))
  (bind _returnvalue (`|CreateWidget` "/Game/BossArena/Widgets/GameModeWidgets/WBP_WaveText.WBP_WaveText_C"))
  (`UserWidget.AddToViewport` _returnvalue 0)
  (`TextBlock.SetText` (`/Game/BossArena/Widgets/GameModeWidgets/WBP_WaveText.TextBlock_WaveText` _returnvalue) (`local.Text Content to Display`))
  (`/Game/BossArena/Widgets/GameModeWidgets/WBP_WaveText.StartCountDown` _returnvalue (`local.InTotalCountDownTime`)))

(fn `UserConstructionScript`)