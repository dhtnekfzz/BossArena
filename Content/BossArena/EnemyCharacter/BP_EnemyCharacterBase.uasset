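; Base enemy character Blueprint for the boss arena, handling dissolve-based spawn and death presentation.
; BeginPlay reverses a timeline to materialize mesh and weapon while playing a random entry montage.
; OnEnemyDied calls a multicast; PlayDeathEffects pauses animation, sets query-only collision, clears UI, async-loads Niagara tinted by the dissolve edge color, then dissolves and destroys character and weapon.
; An unconnected duplicate of the death chain remains.
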(event `self.ReceiveBeginPlay`
  (bind _entry_montages_to_play (`self.Entry Montages to Play`))
  (bind _returnvalue (`PawnCombatComponent.GetCharacterCurrentEquippedWeapon` (`self.EnemyCombatComponent`)))
  (`|ExecutionSequence`
    (:`then_0`
      (`TimelineComponent.SetPlayRate` (`self.EntryRestoreTimeline`) 0.5)
      (bind (_direction _normalizedfloattrack) (`Timeline|EntryRestoreTimeline` :!via `ReverseFromEnd`)
        (:`Update`
          (`MeshComponent.SetScalarParameterValueOnMaterials` (`self.Mesh`) "DissolveAmount" _normalizedfloattrack)
          (`/Engine/EditorBlueprintResources/StandardMacros.IsValid` _returnvalue
            (:`Is Valid`
              (`MeshComponent.SetScalarParameterValueOnMaterials` (`BAWeaponBase.WeaponMesh` _returnvalue) "DissolveAmount" _normalizedfloattrack))))))
    (:`then_1`
      (if (`KismetArrayLibrary.Array_IsNotEmpty` _entry_montages_to_play)
        (`self.PlayAnimMontage` (`KismetArrayLibrary.Array_Random` _entry_montages_to_play))))))

(event `/Game/BossArena/EnemyCharacter/BPI_EnemyDeath.onEnemyDied`
  (params (DissolveNiagaraSystem :type "NiagaraSystem Object Reference"))
  (`self.Multicast_PlayDeathEffects` DissolveNiagaraSystem))

(event `self.BP_PlayDeathEffects`
  (params (NiagaraSystem :type "Object Object Reference"))
  (bind _mesh (`self.Mesh`))
  (bind _returnvalue (`PawnCombatComponent.GetCharacterCurrentEquippedWeapon` (`self.EnemyCombatComponent`)))
  (bind _returnvalue_2 (`PawnCombatComponent.GetCharacterCurrentEquippedWeapon` (`self.EnemyCombatComponent`)))
  (`|ExecutionSequence`
    (:`then_0`
      (set `SkeletalMeshComponent.bPauseAnims` true (`self.Mesh`))
      (`PrimitiveComponent.SetCollisionEnabled` (`self.CapsuleComponent`) "QueryOnly"))
    (:`then_1`
      (`EnemyUIComponent.RemoveEnemyDrawnWidgetsIfAny` (`self.EnemyUIComponent`)))
    (:`then_2`
      (`|LoadAsset` (`|ConvertAsset` NiagaraSystem)
        (:`Completed`
          (bind `_as나이아가라_시스템` (cast `NiagaraSystem` NiagaraSystem)
            (:`then`
              _)
            (:`CastFailed`
              _))
          (bind _returnvalue_3 (`NiagaraFunctionLibrary.SpawnSystemAttached` `_as나이아가라_시스템` (`self.Mesh`) "None" (0.0 0.0 0.0) (struct) "KeepRelativeOffset"))
          (bind _returnvalue_4 (`PrimitiveComponent.CreateDynamicMaterialInstance` _mesh 0 (`PrimitiveComponent.GetMaterial` _mesh 0) "one"))
          (bind _returnvalue_5 (`MaterialInstanceDynamic.K2_GetVectorParameterValue` _returnvalue_4 "DissolveEdgeColor"))
          (`NiagaraComponent.SetNiagaraVariableLinearColor` _returnvalue_3 "DissolveParticleColor" _returnvalue_5)
          (`TimelineComponent.SetPlayRate` (`self.DissolveTimeline`) 0.2)
          (bind (_direction _normalizedfloattrack) (`Timeline|DissolveTimeline`)
            (:`Update`
              (`MeshComponent.SetScalarParameterValueOnMaterials` (`self.Mesh`) "DissolveAmount" _normalizedfloattrack)
              (`/Engine/EditorBlueprintResources/StandardMacros.IsValid` _returnvalue
                (:`Is Valid`
                  (`MeshComponent.SetScalarParameterValueOnMaterials` (`BAWeaponBase.WeaponMesh` _returnvalue) "DissolveAmount" _normalizedfloattrack))))
            (:`Finished`
              (`/Engine/EditorBlueprintResources/StandardMacros.IsValid` _returnvalue_2
                (:`Is Valid`
                  (`self.K2_DestroyActor` _returnvalue_2))
                (:`Is Not Valid`
                  _))
              (`self.K2_DestroyActor`))))))))

(fn `UserConstructionScript`)